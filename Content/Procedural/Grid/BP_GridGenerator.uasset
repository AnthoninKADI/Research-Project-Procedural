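; BP_GridGenerator is a procedural actor that builds a Rows by Columns grid of static mesh components from its construction script.
; GridMaker spaces tiles on X and Y by the Cube's local bounds, whichever mesh each tile receives.
; Each tile uses MeshGrid or, with ObjectRandom set, a random MeshArray entry, plus a random material, and is stored in Tiles.
; BeginPlay does nothing.
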(event EventBeginPlay)

(fn ConstructionScript
  (CallFunction|GridMaker))

(fn GridMaker
  (bind _cube (Variables|Default|GetCube))
  (bind (_min _max) (Components|StaticMesh|GetLocalBounds _cube))
  (Utilities|Array|Clear (Variables|GridParameters|GetTiles))
  (for _index (range 0 (- (Variables|GridParameters|GetRows) 1))
    (for _index_2 (range 0 (- (Variables|GridParameters|GetColumns) 1))
      (bind _returnvalue (AddComponent|AddStaticMeshComponent false (Math|Transform|MakeTransform (Math|Vector|MakeVector (* _index_2 (- (.x _max) (.x _min))) (* _index (- (.y _max) (.y _min))) 0.0) "0, 0, 0" "1.000000,1.000000,1.000000")))
      (if (Variables|GridParameters|GetObject%20Random)
        (Components|StaticMesh|SetStaticMesh _returnvalue (.OutItem (Utilities|Array|Random (Variables|GridParameters|GetMesh%20Array))))
        (else
          (Components|StaticMesh|SetStaticMesh _returnvalue (Variables|GridParameters|GetMesh%20Grid))))
      (Rendering|Material|SetMaterial _returnvalue 0 (.OutItem (Utilities|Array|Random (Variables|GridParameters|GetMaterials%20Array))))
      (Utilities|Array|AddUnique (Variables|GridParameters|GetTiles) _returnvalue))))